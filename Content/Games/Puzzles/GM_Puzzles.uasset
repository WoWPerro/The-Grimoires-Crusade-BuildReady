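; Game mode for the multiplayer puzzle game: the first player possesses a Book pawn and later players possess Knights, spawned at indexed player starts.
; Damage lowers a shared Life, refreshes every pawn's UI and server-travels to GameOver at zero.
; TravelToLevel copies player health into GS_Puzzles and builds a random numbered travel command.
; Score increments on the game state; the health restore/init branch is unconnected.
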(event Custom|TravelToLevel
  (Variables|/Game/Games/Puzzles/GS_Puzzles.GS_Puzzles_C|Setstarted (Variables|Default|GetGS_Puzzlesvar) true)
  (CallFunction|SetLifefromPCtoGS)
  (Development|ExecuteConsoleCommand (Utilities|String|Append "ServerTravel " (Utilities|String|ToString(Integer) (Math|Random|RandomIntegerinRange 1 10))) 0))

(event Custom|SetLife
  (for (_array_element _array_index) (Variables|Default|GetPlayers)
    (Utilities|Array|SetArrayElem (Variables|/Game/Games/Puzzles/GS_Puzzles.GS_Puzzles_C|GetHealth (Variables|Default|GetGS_Puzzlesvar)) _array_index (Variables|/Game/Games/Puzzles/PC_Puzzles.PC_Puzzles_C|GetHealthPC _array_element))))

(event Custom|SetScore
  (bind _gs_puzzlesvar (Variables|Default|GetGS_Puzzlesvar))
  (Variables|/Game/Games/Puzzles/GS_Puzzles.GS_Puzzles_C|SetScore _gs_puzzlesvar (+ (Variables|/Game/Games/Puzzles/GS_Puzzles.GS_Puzzles_C|GetScore _gs_puzzlesvar) 1)))

(event Custom|GameInit
  ;[1 1 1] Se inicializa la vida cuando se carga por primera vez el juego
  (for _array_element (Variables|Default|GetPlayers)
    (Variables|/Game/Games/Puzzles/PC_Puzzles.PC_Puzzles_C|SetHealthPC _array_element 666)
    (Variables|/Game/Games/Puzzles/PC_Puzzles.PC_Puzzles_C|SetScore _array_element 0)))

(event Custom|SetLifeFromPCtoGS
  ;[1 1 1] Guarda las variables del jugador al GS
  (for (_array_element _array_index) (Variables|Default|GetPlayers)
    (Utilities|Array|SetArrayElem (Variables|/Game/Games/Puzzles/GS_Puzzles.GS_Puzzles_C|GetHealth (Variables|Default|GetGS_Puzzlesvar)) _array_index (Variables|/Game/Games/Puzzles/PC_Puzzles.PC_Puzzles_C|GetHealthPC _array_element))))

(event Custom|SetLifeFromGStoPC
  ;[1 1 1] Lodea las variables del GS a los PC
  (for (_array_element _array_index) (Variables|/Game/Games/Puzzles/GS_Puzzles.GS_Puzzles_C|GetHealth (Variables|Default|GetGS_Puzzlesvar))
    (Variables|/Game/Games/Puzzles/PC_Puzzles.PC_Puzzles_C|SetHealthPC (Utilities|Array|Get(acopy) (Variables|Default|GetPlayers) _array_index) _array_element)))

(event Custom|DealDamage
  (Variables|Default|SetLife (- (Variables|Default|GetLife) 1e+01))
  (Default|ModifyUI (Variables|Default|GetBook))
  (for _array_element (Variables|Default|GetKnights)
    (Default|ModifyUI _array_element))
  (Development|PrintString (Utilities|String|ToString(Float) (Variables|Default|GetLife)))
  (if (<= (Variables|Default|GetLife) 0.0)
    (Development|ExecuteConsoleCommand "ServerTravel GameOver" 0)))

(event EventBeginPlay
  (bind _asgs_puzzles (Utilities|Casting|CastToGS_Puzzles (Game|GetGameState)))
  (Variables|Default|SetGS_Puzzlesvar _asgs_puzzles))

(event EventHandleStartingNewPlayer
  (params (NewPlayer :type Player%20Controller%20Object%20Reference))
  (bind _self self)
  (bind _players (Variables|Default|GetPlayers))
  (bind _playerstate (Variables|/Script/Engine.Controller|GetPlayerState NewPlayer))
  (bind _returnvalue (Utilities|Array|Length _players))
  (bind _returnvalue_2 (PlayerState|GetPlayerName _playerstate))
  (bind _returnvalue_3 (- _returnvalue 1))
  (bind _returnvalue_4 (Utilities|String|ToString(Integer) _returnvalue_3))
  (bind _returnvalue_5 (Class|GameModeBase|FindPlayerStart NewPlayer _returnvalue_4))
  (bind _returnvalue_6 (Transformation|GetActorTransform _returnvalue_5))
  (bind _asgs_puzzles (Utilities|Casting|CastToGS_Puzzles (Game|GetGameState)))
  (Variables|Default|SetGS_Puzzlesvar _asgs_puzzles)
  (bind _aspc_puzzles (Utilities|Casting|CastToPC_Puzzles NewPlayer))
  (Utilities|Array|Add (Variables|Default|GetPlayers) _aspc_puzzles)
  (if (not (<= (Utilities|Array|Length (Variables|Default|GetPlayers)) 1))
    (bind _returnvalue_7 (Game|SpawnActorfromClass "/Game/Juanito/Knight_Chr/Player_KnightO.Player_KnightO_C" _returnvalue_6 "Undefined" 0 _returnvalue_2 0))
    (Pawn|Possess NewPlayer _returnvalue_7)
    (Default|SetGM _returnvalue_7 _self)
    (Utilities|Array|Add (Variables|Default|GetKnights) _returnvalue_7)
    (else
      (bind _returnvalue_8 (Game|SpawnActorfromClass "/Game/Juanito/Book_Chr/Player_Book.Player_Book_C" _returnvalue_6 "Undefined" 0 _returnvalue_2 0))
      (Pawn|Possess NewPlayer _returnvalue_8)
      (Default|SetGM _returnvalue_8 _self)
      (Variables|Default|SetBook _returnvalue_8))))

(fn ConstructionScript)