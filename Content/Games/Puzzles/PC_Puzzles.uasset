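; PC_Puzzles is the player controller for the Puzzles game, handling the health HUD and leaving multiplayer sessions.
; On BeginPlay it sets game-only input, aligns control rotation to the controlled pawn and adds a Hud_vida widget to the viewport.
; Tick pushes its HealthPC value into that widget every frame.
; CloseSession destroys the session and, on success, opens the MultiplayerMenu level.
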(event Custom|CloseSession
  (|DestroySession self
    (:OnSuccess
      (Game|OpenLevel(byName) "MultiplayerMenu"))))

(event EventBeginPlay
  (Input|SetInputModeGameOnly self)
  (Pawn|SetControlRotation (Transformation|GetActorRotation (Pawn|GetControlledPawn)))
  (bind _returnvalue (UserInterface|CreateWidget "/Game/Juanito/Knight_Chr/Hud_vida.Hud_vida_C" self))
  (bind _output_get (Variables|Default|SetHudRef _returnvalue))
  (UserInterface|Viewport|AddtoViewport _output_get 0))

(event EventTick
  (params (DeltaSeconds :type Float%20%28single-precision%29))
  (Variables|/Game/Juanito/Knight_Chr/Hud_vida.Hud_vida_C|SetHealth (Variables|Default|GetHudRef) (Variables|Default|GetHealthPC)))

(fn ConstructionScript)